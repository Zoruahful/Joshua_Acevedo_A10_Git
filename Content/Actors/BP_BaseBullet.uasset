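; BP_BaseBullet is a base bullet actor that damages what it overlaps and then destroys itself.
; On BeginPlay it binds to the Collision component's begin overlap and starts a one-shot timer, commented as destroying the bullet after TimeToDestroy.
; The overlap handler applies BaseDamage, crediting the Instigator as damage causer and its controller as event instigator.
; The construction script sets the collision's world scale from the Scale variable.
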(event `self.ReceiveBeginPlay`
  ;[1 1 1] Bullet
  ;;[1 1 1] Collision - Destroy Bullet On Collision
  (add `PrimitiveComponent.OnComponentBeginOverlap` (`self.Collision`) (`|CreateDelegate` :!event `HandleOverlap`))
  ;;[1 1 1] Timer - Destroy Bullet
  (`KismetSystemLibrary.K2_SetTimerDelegate` (`|CreateDelegate` :!event `K2_DestroyActor`) (`self.TimeToDestroy`)))

(event `HandleOverlap`
  (params (OverlappedComponent :type "PrimitiveComponent Object Reference") (OtherActor :type "Actor Object Reference") (OtherComp :type "PrimitiveComponent Object Reference") (OtherBodyIndex :type Integer) (bFromSweep :type Boolean) (SweepResult :type "HitResult Structure (by ref)"))
  ;[1 1 1] Bullet
  ;;[1 1 1] Collision - Destroy Bullet On Collision
  (`GameplayStatics.ApplyDamage` OtherActor (`self.BaseDamage`) (`self.GetInstigatorController`) (`self.GetInstigator`))
  (`self.K2_DestroyActor`))

(fn `UserConstructionScript`
  (`SceneComponent.SetWorldScale3D` (`self.Collision`) (`self.Scale`)))