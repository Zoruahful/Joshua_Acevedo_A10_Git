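; Player character Blueprint that handles movement, camera look and attack input.
; Movement axes follow the controller's yaw only, look axes add yaw and pitch, and the Attack press calls CharacterAttack.
; On BeginPlay it creates the HUD widget for its PlayerController and binds to the health component's hurt and death events.
; Without a PlayerController it prints a warning and destroys itself.
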(event `self.ReceiveBeginPlay`
  (bind _bp_healthcomponent (`self.BP_HealthComponent`))
  ;[1 1 1] Default
  (`parent.ReceiveBeginPlay`)
  ;[1 1 1] Week 1 Lecture 3   ----> Complete this
  (bind _asplayer_controller (cast `PlayerController` (`self.GetController`))
    (:`then`
      (bind _returnvalue (`|CreateWidget` (`self.WidgetClass`) _asplayer_controller))
      (bind _output_get (set `self.HUDWidget` _returnvalue))
      (`UserWidget.AddToViewport` _output_get 0)
      (add `/Game/Components/BP_HealthComponent.OnHurt` _bp_healthcomponent (`|CreateDelegate` (`self.HUDWidget`) :!event `SetHealth`))
      (add `/Game/Components/BP_HealthComponent.OnDead` _bp_healthcomponent (`|CreateDelegate` (`self.HUDWidget`) :!event `SetHealth`)))
    (:`CastFailed`
      (`KismetSystemLibrary.PrintString` "Need A Player Controller")
      (`self.K2_DestroyActor`))))

(event `InputAction|Attack`
  (params (Key :type "Key Structure"))
  ;[1 1 1] Shoot
  (:`Pressed`
    (`self.Character Attack`)))

(event `InputAxis|Forward`
  (params (AxisValue :type "Float (single-precision)"))
  (bind (_returnvalue_roll _returnvalue_pitch _returnvalue_yaw) (`KismetMathLibrary.BreakRotator` (`self.GetControlRotation`)))
  ;[1 1 1] Movement & Camera
  ;;[1 1 1] Forward & Back    DONE!!!
  (`self.AddMovementInput` (`KismetMathLibrary.GetForwardVector` (`KismetMathLibrary.MakeRotator` 0.0 0.0 _returnvalue_yaw)) AxisValue))

(event `InputAxis|TurnTo`
  (params (AxisValue :type "Float (single-precision)"))
  ;[1 1 1] Movement & Camera
  ;;[1 1 1] Camera - Mouse Input  DONE!!!
  (`self.AddControllerYawInput` AxisValue))

(event `InputAxis|Right`
  (params (AxisValue :type "Float (single-precision)"))
  (bind (_returnvalue_roll _returnvalue_pitch _returnvalue_yaw) (`KismetMathLibrary.BreakRotator` (`self.GetControlRotation`)))
  ;[1 1 1] Movement & Camera
  ;;[1 1 1] Left & Right  DONE!!!
  (`self.AddMovementInput` (`KismetMathLibrary.GetRightVector` (`KismetMathLibrary.MakeRotator` 0.0 0.0 _returnvalue_yaw)) AxisValue))

(event `InputAxis|LookUp`
  (params (AxisValue :type "Float (single-precision)"))
  ;[1 1 1] Movement & Camera
  ;;[1 1 1] Camera - Mouse Input  DONE!!!
  (`self.AddControllerPitchInput` AxisValue))

(fn `UserConstructionScript`
  (`parent.UserConstructionScript`))