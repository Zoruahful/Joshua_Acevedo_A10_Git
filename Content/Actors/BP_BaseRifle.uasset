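; Base rifle weapon actor that fires projectiles on behalf of the Pawn that is its parent actor.
; On BeginPlay it caches that parent Pawn, printing a warning if none is found.
; Attack spawns the bullet class at a skeletal mesh socket along the Pawn's base aim rotation, with the Pawn as instigator.
; A Busy flag and one-shot timer gate the fire rate, with FinshAttack clearing the flag.
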(event `self.ReceiveBeginPlay`
  (bind _aspawn (cast `Pawn` (`self.GetParentActor`))
    (:`then`
      (set `self.parentPawn` _aspawn))
    (:`CastFailed`
      (`KismetSystemLibrary.PrintString` "We Need a pawn to use this weapon"))))

(fn `Attack`
  ;[1 1 1] Bullet Spawn
  (if (`self.CanAttack`)
    (`|SpawnActorFromClass` (`self.BulletClass`) (`KismetMathLibrary.MakeTransform` (`SceneComponent.GetSocketLocation` (`self.SkeletalMesh`) (`self.SocketName`)) (`Pawn.GetBaseAimRotation` (`self.parentPawn`))) "Undefined" "OverrideRootScale" null (`self.parentPawn`))
    (set `self.Busy` true)
    (`KismetSystemLibrary.K2_SetTimerDelegate` (`|CreateDelegate` :!event `FinshAttack`) 2.0)))

(fn `CanAttack`
  (returns (Yes :type Boolean))
  (return (not (`self.Busy`))))

(fn `FinshAttack`
  (set `self.Busy` false))

(fn `UserConstructionScript`)