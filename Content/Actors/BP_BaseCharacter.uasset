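; Base character Blueprint that carries a rifle and can attack with it.
; On BeginPlay it spawns WeaponClass through a child actor component and caches it as a BP_BaseRifle, destroying itself if that cast fails.
; It then caches its ABP_Character anim instance and binds health component hurt and death events, with hurt only printing the amount.
; CharacterAttack triggers the weapon's attack and the fire animation.
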(event `self.ReceiveBeginPlay`
  (bind _weaponchildactorcomponent (`self.WeaponChildActorComponent`))
  (bind _bp_healthcomponent (`self.BP_HealthComponent`))
  ;[1 1 1] Spawn Weapon
  (`ChildActorComponent.SetChildActorClass` _weaponchildactorcomponent (`self.WeaponClass`))
  (bind _asbp_base_rifle (cast `/Game/Actors/BP_BaseRifle` (`ChildActorComponent.ChildActor` _weaponchildactorcomponent))
    (:`then`
      (set `self.CurrentWeapon` _asbp_base_rifle)
      (bind _asabp_character (cast `/Game/Core/Art/ABP_Character` (`SkeletalMeshComponent.GetAnimInstance` (`self.Mesh`)))
        (:`then`
          (set `self.AnimBP` _asabp_character)
          (add `/Game/Components/BP_HealthComponent.OnHurt` _bp_healthcomponent (delegate `Testing`))
          (add `/Game/Components/BP_HealthComponent.OnDead` _bp_healthcomponent (`|CreateDelegate` :!event `Testing`)))
        (:`CastFailed`
          (`KismetSystemLibrary.PrintString` "We have to set our animation to the right type"))))
    (:`CastFailed`
      (`KismetSystemLibrary.PrintString` "There is no weapon will crash")
      (`self.K2_DestroyActor`))))

(event `Testing`
  (params (Amount :type "Float (double-precision)"))
  ;[1 1 1] Spawn Weapon
  (`KismetSystemLibrary.PrintString` (`KismetStringLibrary.Conv_DoubleToString` Amount)))

(fn `Character Attack`
  (`/Game/Actors/BP_BaseRifle.Attack` (`self.CurrentWeapon`))
  (`/Game/Core/Art/ABP_Character.Play Fire Animation` (`self.AnimBP`)))

(fn `UserConstructionScript`)